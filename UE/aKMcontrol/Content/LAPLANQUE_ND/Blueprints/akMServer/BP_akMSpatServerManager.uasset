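; Manager actor for the external akM spatialization audio server, which it launches through a C++ call on BeginPlay and controls over OSC.
; Heartbeat messages mark the server alive and restart a watchdog timer that clears the flag when they stop.
; Functions send quit and system gain commands through the BP_OSCInterface found in the level.
; System acknowledgements are parsed, and gain values are printed.
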(event EventOnAckMessageReceived
  (params (OSCMessage :type OSC%20Message%20Structure))
  (bind _returnvalue (Class|OSCManager|GetOSCMessageAddress OSCMessage))
  (bind _returnvalue_2 (Class|OSCManager|ConvertStringtoOSCAddress "/*/*/system/*"))
  (bind _returnvalue_3 (Class|OSCManager|OSCAddressPathMatchesPattern _returnvalue_2 _returnvalue))
  (if _returnvalue_3
    (CallFunction|ProcessAckSystem OSCMessage)))

(event EventOnServerStatusMessageReceived
  (params (OSCMessage :type OSC%20Message%20Structure))
  (bind _returnvalue (Class|OSCManager|GetOSCMessageAddress OSCMessage))
  (bind _returnvalue_2 (Class|OSCManager|ConvertStringtoOSCAddress "/*/*/heartbeat"))
  (bind _returnvalue_3 (Class|OSCManager|OSCAddressPathMatchesPattern _returnvalue_2 _returnvalue))
  (if _returnvalue_3
    (if (Variables|Default|GetbServerIsStarting)
      (Variables|Default|SetbServerIsStarting false))
    (Utilities|Time|ClearandInvalidateTimerbyHandle (Variables|Default|GetServerAliveTimer))
    (Variables|Default|SetbIsServerAlive true)
    (bind _returnvalue_4 (Utilities|Time|SetTimerbyFunctionName 0 "ResetServerAliveStatus" (Variables|Default|GetServerAliveTimerDuration)))
    (Variables|Default|SetServerAliveTimer _returnvalue_4)))

(event EventBeginPlay
  (bind _outactors (Actor|GetAllActorsOfClass "/Game/LAPLANQUE_ND/Blueprints/OSC/BP_OSCInterface.BP_OSCInterface_C"))
  (Variables|Default|SetOSCInterface (Utilities|Array|Get(acopy) _outactors))
  (Class|AkMSpatServerManager|StartSpatServer) ; Implemented in C++
  (Variables|Default|SetbIsServerAlive false)
  (bind _returnvalue (Utilities|Time|SetTimerbyFunctionName 0 "ResetServerAliveStatus" (Variables|Default|GetServerAliveTimerDuration)))
  (Variables|Default|SetServerAliveTimer _returnvalue))

(fn ConstructionScript)

(fn ResetServerAliveStatus
  (Variables|Default|SetbIsServerAlive false))

(fn StopSpatServer
  (bind _oscinterface (Variables|Default|GetOSCInterface)
    (:then
      (bind _returnvalue (Class|OSCManager|ConvertStringtoOSCAddress "/quit"))
      (bind _returnvalue_2 (Class|OSCManager|SetOSCMessageAddress (Utilities|Struct|MakeOSCMessage) _returnvalue))
      (Class|OSCClient|SendOSCMessage (Variables|/Game/LAPLANQUE_ND/Blueprints/OSC/BP_OSCInterface.BP_OSCInterface_C|GetakMServer-Sender _oscinterface) _returnvalue_2))
    (:else)))

(fn SetSystemGain
  (params (Gain :type Float%20%28double-precision%29))
  (bind _returnvalue (Utilities|String|MakeLiteralString "/system/gain"))
  (bind _oscinterface (Variables|Default|GetOSCInterface)
    (:then
      (bind _returnvalue_2 (Class|OSCManager|ConvertStringtoOSCAddress _returnvalue))
      (bind _returnvalue_3 (Class|OSCManager|SetOSCMessageAddress (Utilities|Struct|MakeOSCMessage) _returnvalue_2))
      (bind _returnvalue_4 (Class|OSCManager|AddFloat _returnvalue_3 Gain))
      (Class|OSCClient|SendOSCMessage (Variables|/Game/LAPLANQUE_ND/Blueprints/OSC/BP_OSCInterface.BP_OSCInterface_C|GetakMServer-Sender _oscinterface) _returnvalue_4)
      (Development|PrintString (Utilities|String|Append "SEND: " _returnvalue ", VALUE: " (Utilities|String|ToString(Float) Gain)) false))
    (:else)))

(fn ProcessAckSystem
  (params (OSCMessage :type OSC%20Message%20Structure))
  (bind _output_get (LocalVariables|SetMessage OSCMessage))
  (bind _returnvalue (Class|OSCManager|GetOSCMessageAddress _output_get))
  (Utilities|FlowControl|Sequence
    (:then_0
      (bind _returnvalue_2 (Class|OSCManager|GetOSCAddressFullPath _returnvalue))
      (LocalVariables|SetShortenedAddress (.RightS (Utilities|String|Split _returnvalue_2 "/akMserver/ack"))))
    (:then_1
      (bind _returnvalue_3 (Class|OSCManager|GetOSCAddressMethod _returnvalue))
      (switch string _returnvalue_3
        (:gain
          (bind _value (Class|OSCManager|GetFloat (LocalVariables|GetMessage)))
          (Development|PrintString (Utilities|String|Append "ACK: " (LocalVariables|GetShortenedAddress) ", VALUE: " (Utilities|String|ToString(Float) _value)) false))))))