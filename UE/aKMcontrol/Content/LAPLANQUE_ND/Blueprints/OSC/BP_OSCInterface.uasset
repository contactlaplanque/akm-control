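; BP_OSCInterface is the OSC bridge between the game and an external akM spatialization server.
; On BeginPlay it opens an OSC server on all interfaces and creates a client that targets localhost.
; Incoming status and ack messages under /akMserver are matched by address pattern and broadcast to every actor implementing BPI_akMSpatServer.
; The sender client is created and stored, but this Blueprint sends nothing itself.
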(event Custom|OnServerAckMessage
  (params (AddressPattern :type OSC%20Address%20Structure%20%28by%20ref%29) (Message :type OSC%20Message%20Structure%20%28by%20ref%29) (IPAddress :type String) (Port :type Integer))
  (bind _outactors (Actor|GetAllActorswithInterface "/Game/LAPLANQUE_ND/Blueprints/Interfaces/BPI_akMSpatServer.BPI_akMSpatServer_C"))
  (for _array_element _outactors
    (Class|BPIAkMSpatServer|OnAckMessageReceived(Message) _array_element Message)))

(event Custom|OnServerStatusMessage
  (params (AddressPattern :type OSC%20Address%20Structure%20%28by%20ref%29) (Message :type OSC%20Message%20Structure%20%28by%20ref%29) (IPAddress :type String) (Port :type Integer))
  (bind _outactors (Actor|GetAllActorswithInterface "/Game/LAPLANQUE_ND/Blueprints/Interfaces/BPI_akMSpatServer.BPI_akMSpatServer_C"))
  (for _array_element _outactors
    (Class|BPIAkMSpatServer|OnServerStatusMessageReceived(Message) _array_element Message)))

(event EventBeginPlay
  (Utilities|FlowControl|Sequence
    (:then_0
      (bind _returnvalue (Class|OSCManager|CreateOSCServer "0.0.0.0" 23444 false true "OSCListener-akMServer" "BP_OSCInterface"))
      (Variables|Default|SetakMServer-Listener _returnvalue)
      (bind _returnvalue_2 (Class|OSCManager|ConvertStringtoOSCAddress "/akMserver/status/*"))
      (Class|OSCServer|BindEventtoonOSCAddressPatternMatchesPath (Variables|Default|GetakMServer-Listener) _returnvalue_2 (delegate Custom|OnServerStatusMessage))
      (bind _returnvalue_3 (Class|OSCManager|ConvertStringtoOSCAddress "/akMserver/ack/*"))
      (Class|OSCServer|BindEventtoonOSCAddressPatternMatchesPath (Variables|Default|GetakMServer-Listener) _returnvalue_3 (delegate Custom|OnServerAckMessage)))
    (:then_1
      (bind _returnvalue_4 (Class|OSCManager|CreateOSCClient "127.0.0.1" 23446 "OSCSender-akMServer" "BP_OSCInterface"))
      (Variables|Default|SetakMServer-Sender _returnvalue_4))))

(fn ConstructionScript)