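; BP_akMColumn is a column actor whose bottom, middle and top labels turn to face the player character's camera.
; On BeginPlay it caches the first BP_akMCharacter found in the level.
; Each Tick, while that reference is valid, it applies a yaw-only billboard: the look-at yaw from camera to column mesh, flipped 180 degrees, becomes all three labels' world rotation, keeping them upright.
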(event EventTick
  (params (DeltaSeconds :type Float%20%28single-precision%29))
  (bind _akmcharacter (Variables|Default|GetakMCharacter)
    (:then
      (Transformation|SetWorldRotation (Variables|Default|GetLabelBottom) (Math|Rotator|MakeRotator 0.0 0.0 (+ (.yaw (Math|Rotator|FindLookatRotation (Transformation|GetWorldLocation (Variables|/Game/LAPLANQUE_ND/Character/BP_akMCharacter.BP_akMCharacter_C|GetCamera _akmcharacter)) (Transformation|GetWorldLocation (Variables|Debug|GetStaticMeshComponent)))) 1.8e+02)) false false)
      (Transformation|SetWorldRotation (Variables|Default|GetLabelMiddle) (Math|Rotator|MakeRotator 0.0 0.0 (+ (.yaw (Math|Rotator|FindLookatRotation (Transformation|GetWorldLocation (Variables|/Game/LAPLANQUE_ND/Character/BP_akMCharacter.BP_akMCharacter_C|GetCamera _akmcharacter)) (Transformation|GetWorldLocation (Variables|Debug|GetStaticMeshComponent)))) 1.8e+02)) false false)
      (Transformation|SetWorldRotation (Variables|Default|GetLabelTop) (Math|Rotator|MakeRotator 0.0 0.0 (+ (.yaw (Math|Rotator|FindLookatRotation (Transformation|GetWorldLocation (Variables|/Game/LAPLANQUE_ND/Character/BP_akMCharacter.BP_akMCharacter_C|GetCamera _akmcharacter)) (Transformation|GetWorldLocation (Variables|Debug|GetStaticMeshComponent)))) 1.8e+02)) false false))
    (:else)))

(event EventBeginPlay
  (bind _outactors (Actor|GetAllActorsOfClass "/Game/LAPLANQUE_ND/Character/BP_akMCharacter.BP_akMCharacter_C"))
  (Variables|Default|SetakMCharacter (Utilities|Array|Get(acopy) _outactors)))

(fn ConstructionScript)