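; Translate gizmo that selects Source actors and drags them along the X, Y or Z axis.
; Mouse position in the main UI view becomes a UV, deprojected through the character's SceneCapture2D for line-trace picking.
; Dragging pauses camera movement and projects mouse motion at grab distance onto the handle's forward vector, moving gizmo and source.
; A looping timer updates hover highlights; Tick hides the gizmo when nothing is selected.
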(event Custom|OnHoverUpdateTimer
  (CallFunction|UpdateHoverMaterials))

(event EventBeginPlay
  (Input|EnableInput (Game|GetPlayerController 0))
  (bind _outactors (Actor|GetAllActorsOfClass "/Game/LAPLANQUE_ND/Character/BP_akMCharacter.BP_akMCharacter_C"))
  (Variables|Default|SetakMCharacter (Utilities|Array|Get(acopy) _outactors))
  (Utilities|Time|SetTimerbyEvent (delegate Custom|OnHoverUpdateTimer) 0.1 true true))

(event EventTick
  (params (DeltaSeconds :type Float%20%28single-precision%29))
  (bind _uv (CallFunction|GetUVfromMouseonSceneCapture))
  (bind _akmcharacter (Variables|Default|GetakMCharacter))
  (bind _defaultsceneroot (Variables|Default|GetDefaultSceneRoot))
  (bind _scenecapturecomponent2d (Variables|/Game/LAPLANQUE_ND/Character/BP_akMCharacter.BP_akMCharacter_C|GetSceneCaptureComponent2D _akmcharacter))
  (bind (_worldposition _worlddirection) (Class|GameplayStatics|DeprojectSceneCaptureComponenttoWorld _scenecapturecomponent2d _uv))
  (Variables|Default|GetSelectedSource
    (:then
      (Rendering|SetVisibility _defaultsceneroot true true)
      (Collision|SetActorEnableCollision true)
      (if (Variables|Default|GetIsDragging)
        (bind _draggedhandlecomponent (Variables|Default|GetDraggedHandleComponent)
          (:then
            (Rendering|Material|SetMaterial _draggedhandlecomponent 0 "/Game/LAPLANQUE_ND/MaterialsLibrary/Gizmo/M_GizmoHover.M_GizmoHover")
            (Transformation|SetWorldLocation (Variables|Default|GetGizmoRoot) (+ (Variables|Default|GetGizmoLocationWhenClicked) (Math|Vector|NegateVector (Math|Vector|ProjectVectorontoVector (- (Variables|Default|GetDragLocation) (+ _worldposition (* _worlddirection (Variables|Default|GetDistanceToGrab)))) (Math|Vector|GetForwardVector _draggedhandlecomponent)))) false false)
            (bind _selectedsource (Variables|Default|GetSelectedSource)
              (:then
                (Class|Source|SetPosition _selectedsource (+ (Variables|Default|GetGizmoLocationWhenClicked) (Math|Vector|NegateVector (Math|Vector|ProjectVectorontoVector (- (Variables|Default|GetDragLocation) (+ _worldposition (* _worlddirection (Variables|Default|GetDistanceToGrab)))) (Math|Vector|GetForwardVector _draggedhandlecomponent))))))
              (:else)))
          (:else))))
    (:else
      (Rendering|SetVisibility _defaultsceneroot false true)
      (Collision|SetActorEnableCollision false))))

(event Input|MouseEvents|LeftMouseButton
  (params (Key :type Key%20Structure :default "None"))
  (:Pressed
    (bind _hit_result (CallFunction|PerformLineTraceonSceneCaptureView))
    (Variables|Default|SetDistanceToGrab (.Distance (Collision|BreakHitResult _hit_result)))
    (if (== (Utilities|GetClass (.HitActor (Collision|BreakHitResult _hit_result))) "/Script/aKMcontrol.Source")
      (bind _assource (Utilities|Casting|CastToSource (.HitActor (Collision|BreakHitResult _hit_result))))
      (CallFunction|SelectNewSource _assource)
      (elif (.IsValidAxis (CallFunction|GetDraggedHandlefromHitComponent (.HitComponent (Collision|BreakHitResult _hit_result))))
        (Variables|Default|SetIsDragging true)
        (Variables|Default|SetDraggedHandleComponent (.HitComponent (Collision|BreakHitResult _hit_result)))
        (Variables|Default|SetDragLocation (.Location (Collision|BreakHitResult _hit_result)))
        (Variables|/Game/LAPLANQUE_ND/Character/BP_akMCharacter.BP_akMCharacter_C|SetbCameraMovementActive (Variables|Default|GetakMCharacter) false)
        (Variables|Default|SetGizmoLocationWhenClicked (Transformation|GetWorldLocation (Variables|Default|GetGizmoRoot)))
        (else
          (Variables|Default|SetIsDragging false)
          (CallFunction|ResetSelection)))))
  (:Released
    (Variables|Default|SetDraggedHandleComponent 0)
    (Variables|Default|SetIsDragging false)
    (Variables|/Game/LAPLANQUE_ND/Character/BP_akMCharacter.BP_akMCharacter_C|SetbCameraMovementActive (Variables|Default|GetakMCharacter) true)
    (CallFunction|ResetHandleMaterials)))

(event Input|KeyboardEvents|C
  (params (Key :type Key%20Structure :default "None"))
  (:Pressed
    (CallFunction|ResetSelection)))

(fn ConstructionScript)

(fn GetDraggedHandlefromHitComponent
  (params (Component :type Primitive%20Component%20Object%20Reference))
  (bind _output_get (LocalVariables|SetHitComponent Component))
  (if (== _output_get (Variables|Default|GetHandleX))
    (return "NewEnumerator0" true)
    (elif (== (LocalVariables|GetHitComponent) (Variables|Default|GetHandleY))
      (return "NewEnumerator1" true)
      (elif (== (LocalVariables|GetHitComponent) (Variables|Default|GetHandleZ))
        (return "NewEnumerator2" true)
        (else
          (return "NewEnumerator0" false))))))

(fn GetUVfromMouseonSceneCapture
  (bind _returnvalue (Game|GetPlayerController 0))
  (bind _akmcharacter (Variables|Default|GetakMCharacter))
  (bind (_locationx _locationy) (Class|WidgetLayoutLibrary|GetMousePositionScaledbyDPI _returnvalue))
  (bind _mainui (Variables|/Game/LAPLANQUE_ND/Character/BP_akMCharacter.BP_akMCharacter_C|GetMainUI _akmcharacter))
  (bind _mainviewlocaltopleft (Variables|/Game/LAPLANQUE_ND/UI/WBP_MainUI.WBP_MainUI_C|GetMainViewLocalTopLeft _mainui))
  (bind _mainviewlocalsize (Variables|/Game/LAPLANQUE_ND/UI/WBP_MainUI.WBP_MainUI_C|GetMainViewLocalSize _mainui))
  (return (Math|Vector2D|MakeVector2D (/ (Math|Float|Clamp(Float) (- _locationx (.x _mainviewlocaltopleft)) 0.0 (.x _mainviewlocalsize)) (.x _mainviewlocalsize)) (/ (Math|Float|Clamp(Float) (- _locationy (.y _mainviewlocaltopleft)) 0.0 (.y _mainviewlocalsize)) (.y _mainviewlocalsize)))))

(fn PerformLineTraceonSceneCaptureView
  (bind _uv (CallFunction|GetUVfromMouseonSceneCapture))
  (bind _akmcharacter (Variables|Default|GetakMCharacter))
  (bind _scenecapturecomponent2d (Variables|/Game/LAPLANQUE_ND/Character/BP_akMCharacter.BP_akMCharacter_C|GetSceneCaptureComponent2D _akmcharacter))
  (bind (_worldposition _worlddirection) (Class|GameplayStatics|DeprojectSceneCaptureComponenttoWorld _scenecapturecomponent2d _uv))
  (if (Variables|/Game/LAPLANQUE_ND/UI/WBP_MainUI.WBP_MainUI_C|GetbIsMouseOverMainView (Variables|/Game/LAPLANQUE_ND/Character/BP_akMCharacter.BP_akMCharacter_C|GetMainUI (Variables|Default|GetakMCharacter)))
    (bind _outhit (Collision|LineTraceByChannel _worldposition (+ _worldposition (* _worlddirection 5e+04)) "TraceTypeQuery2" true (Utilities|Array|MakeArray (Variables|Default|GetakMCharacter)) "None" false))
    (return _outhit)))

(fn UpdateHoverMaterials
  (if (not (Variables|Default|GetIsDragging))
    (bind _hit_result (CallFunction|PerformLineTraceonSceneCaptureView))
    (LocalVariables|SetHitActor (.HitActor (Collision|BreakHitResult _hit_result)))
    (LocalVariables|SetHitComponent (.HitComponent (Collision|BreakHitResult _hit_result)))
    (Utilities|FlowControl|Sequence
      (:then_0
        (if (== (Utilities|GetClass (LocalVariables|GetHitActor)) "/Script/aKMcontrol.Source")
          (bind _assource (Utilities|Casting|CastToSource (LocalVariables|GetHitActor)))
          (bind _output_get (Variables|Default|SetHoveredSource _assource))
          (CallFunction|SetSourceHoverMaterial _output_get)
          (else
            (bind _hoveredsource (Variables|Default|GetHoveredSource)
              (:then
                (CallFunction|ResetSourceHoverMaterial _hoveredsource)
                (Variables|Default|SetHoveredSource 0))
              (:else)))))
      (:then_1
        (Variables|Default|GetSelectedSource
          (:then
            (if (.IsValidAxis (CallFunction|GetDraggedHandlefromHitComponent (LocalVariables|GetHitComponent)))
              (switch Utilities|FlowControl|Switch|SwitchonE_GizmoAxes (.DraggedAxis (CallFunction|GetDraggedHandlefromHitComponent (LocalVariables|GetHitComponent)))
                (:NewEnumerator0
                  (Rendering|Material|SetMaterial (Variables|Default|GetHandleX) 0 "/Game/LAPLANQUE_ND/MaterialsLibrary/Gizmo/M_GizmoHover.M_GizmoHover"))
                (:NewEnumerator1
                  (Rendering|Material|SetMaterial (Variables|Default|GetHandleY) 0 "/Game/LAPLANQUE_ND/MaterialsLibrary/Gizmo/M_GizmoHover.M_GizmoHover"))
                (:NewEnumerator2
                  (Rendering|Material|SetMaterial (Variables|Default|GetHandleZ) 0 "/Game/LAPLANQUE_ND/MaterialsLibrary/Gizmo/M_GizmoHover.M_GizmoHover")))
              (else
                (CallFunction|ResetHandleMaterials))))
          (:else))))))

(fn ResetHandleMaterials
  (Rendering|Material|SetMaterial (Variables|Default|GetHandleX) 0 "/Game/LAPLANQUE_ND/MaterialsLibrary/Gizmo/M_GizmoX.M_GizmoX")
  (Rendering|Material|SetMaterial (Variables|Default|GetHandleY) 0 "/Game/LAPLANQUE_ND/MaterialsLibrary/Gizmo/M_GizmoY.M_GizmoY")
  (Rendering|Material|SetMaterial (Variables|Default|GetHandleZ) 0 "/Game/LAPLANQUE_ND/MaterialsLibrary/Gizmo/M_GizmoZ.M_GizmoZ"))

(fn SetSourceHoverMaterial
  (params (Source :type Source%20Object%20Reference))
  (Rendering|Material|SetVectorParameterValue (Variables|/Script/aKMcontrol.Source|GetSourceInnerMID Source) "Color" "(R=1.000000,G=1.000000,B=0.000000,A=1.000000)" :!class /Script/Engine.MaterialInstanceDynamic)
  (Rendering|Material|SetVectorParameterValue (Variables|/Script/aKMcontrol.Source|GetSourceOuterMID Source) "TintColor" "(R=1.000000,G=1.000000,B=0.000000,A=1.000000)" :!class /Script/Engine.MaterialInstanceDynamic)
  (Rendering|Components|TextRender|SetTextRenderColor (Variables|/Script/aKMcontrol.Source|GetSourceLabel Source) (Math|Color|MakeColor 0 1 1 1)))

(fn ResetSourceHoverMaterial
  (params (Source :type Source%20Object%20Reference))
  (bind _color (Variables|/Script/aKMcontrol.Source|GetColor Source))
  (Rendering|Material|SetVectorParameterValue (Variables|/Script/aKMcontrol.Source|GetSourceInnerMID Source) "Color" (Math|Conversions|ToLinearColor(Color) _color) :!class /Script/Engine.MaterialInstanceDynamic)
  (Rendering|Material|SetVectorParameterValue (Variables|/Script/aKMcontrol.Source|GetSourceOuterMID Source) "TintColor" (Math|Conversions|ToLinearColor(Color) _color) :!class /Script/Engine.MaterialInstanceDynamic)
  (Rendering|Components|TextRender|SetTextRenderColor (Variables|/Script/aKMcontrol.Source|GetSourceLabel Source) _color))

(fn SelectNewSource
  (params (New%20Source :type Source%20Object%20Reference))
  (bind _output_get (Variables|Default|SetSelectedSource New%20Source))
  (Transformation|SetWorldLocation (Variables|Default|GetGizmoRoot) (Variables|/Script/aKMcontrol.Source|GetPosition _output_get) false true))

(fn ResetSelection
  (Variables|Default|SetSelectedSource 0))