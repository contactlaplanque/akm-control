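; Manager for a pool of sources that runs and resets two demos in response to bound event dispatchers.
; Demo 1 activates one colored source and moves it around a circle with a looping timer.
; Demo 2 spawns a Niagara system that exports particle data back to this Blueprint, driving the positions of five pooled sources with random radii.
; Reset deactivates all sources, clears the timer and destroys the Niagara component.
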(event Custom|OnResetSourcesDemo_Event
  (CallFunction|ResetDemos))

(event Custom|OnSourcesDemo1_Event
  (CallFunction|StartDemo1))

(event Custom|OnSourcesDemo2_Event
  (CallFunction|StartDemo2))

(event Custom|StartDemo1
  (Class|SourcesManager|ActivateSourcebyID 1)
  (bind _output_get (Variables|Default|SetDemo1Source (Utilities|Array|Get(acopy) (Variables|Default|GetSources))))
  (Class|Source|SetRadius _output_get (Variables|Default|GetDemo1SourceRadius))
  (Class|Source|SetColor (Variables|Default|GetDemo1Source) (Math|Conversions|ToColor(LinearColor) (Utilities|Struct|MakeLinearColor 1.0 0.31 0.2 0.1)))
  (Class|Source|SetA (Variables|Default|GetDemo1Source) (Variables|Default|GetDemo1Source1))
  (Variables|Default|SetDemo1Source1Position (Math|Vector|MakeVector (Variables|Default|GetDemo1SourceRadius) 0.0 (Variables|Default|GetDemo1TrajectoryHeight)))
  (Variables|Default|SetDemo1CurrentAngle 0.0)
  (bind _returnvalue (Utilities|Time|SetTimerbyEvent (delegate Custom|UpdateDemo1) 0.01 true true))
  (Variables|Default|SetDemo1UpdateTimer _returnvalue))

(event Custom|UpdateDemo1
  (bind _demo1trajectoryradius (Variables|Default|GetDemo1TrajectoryRadius))
  (bind _output_get (Variables|Default|SetDemo1CurrentAngle (+ (Variables|Default|GetDemo1Speed) (Variables|Default|GetDemo1CurrentAngle))))
  (bind _output_get_2 (Variables|Default|SetDemo1Source1Position (Math|Vector|MakeVector (* _demo1trajectoryradius (Math|Trig|Cos(Degrees) _output_get)) (* _demo1trajectoryradius (Math|Trig|Sin(Degrees) _output_get)) (Variables|Default|GetDemo1TrajectoryHeight))))
  (Class|Source|SetPosition (Variables|Default|GetDemo1Source) _output_get_2))

(event Custom|StartDemo2
  (bind _returnvalue (Niagara|SpawnSystematLocation "/Game/LAPLANQUE_ND/DemoSources/NS_Demo2.NS_Demo2" "0.000000,0.000000,150.000000"))
  (bind _output_get (Variables|Default|SetDemo2NiagaraSystem _returnvalue))
  (Class|NiagaraComponent|SetVariableObject _output_get "UserCallback" self)
  (for _index (range 0 4)
    (bind _returnvalue_2 (Class|SourcesManager|ActivateNextInactiveSource))
    (Utilities|Array|Add (Variables|Default|GetDemo2Sources) _returnvalue_2)
    (Class|Source|SetRadius _returnvalue_2 (Math|Random|RandomFloatinRange 1e+02 2e+02))))

(event EventBeginPlay
  (EventDispatchers|AssignOnResetSourcesDemo (delegate Custom|OnResetSourcesDemo_Event))
  (EventDispatchers|AssignOnSourcesDemo1 (delegate Custom|OnSourcesDemo1_Event))
  (EventDispatchers|AssignOnSourcesDemo2 (delegate Custom|OnSourcesDemo2_Event)))

(event EventParticleData
  (params (Data :type Array%20of%20Basic%20Particle%20Data%20Structures) (NiagaraSystem :type Niagara%20System%20Object%20Reference) (SimulationPositionOffset :type Vector%20%28by%20ref%29 :default "0, 0, 0"))
  (for (_array_element _array_index) Data
    (Utilities|IsValid (Utilities|Array|Get(acopy) (Variables|Default|GetDemo2Sources) _array_index)
      (:Is%20Valid
        (Class|Source|SetPosition (Utilities|Array|Get(acopy) (Variables|Default|GetDemo2Sources) _array_index) (.Position (Utilities|Struct|BreakBasicParticleData _array_element)))))))

(fn ConstructionScript)

(fn ResetDemos
  (for _array_element (Variables|Default|GetSources)
    (Class|Source|SetActive _array_element false))
  (Utilities|Time|ClearandInvalidateTimerbyHandle (Variables|Default|GetDemo1UpdateTimer))
  (Utilities|Array|Clear (Variables|Default|GetDemo2Sources))
  (bind _demo2niagarasystem (Variables|Default|GetDemo2NiagaraSystem)
    (:then
      (Components|DestroyComponent _demo2niagarasystem)
      (Variables|Default|SetDemo2NiagaraSystem 0))
    (:else)))