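; Player camera character that moves on three axes, with hold-to-look rotation and smoothed spring-arm zoom via Enhanced Input.
; On BeginPlay it creates WBP_MainUI, shows the cursor in Game and UI input mode and finds the level's BP_ImGUI actor.
; Movement, look and zoom respond only while the mouse is over the UI's main view.
; Tick copies that view's geometry to ImGUI and enables ImGui input when the mouse is outside it.
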(event Input|EnhancedActionEvents|EnhancedInputActionIA_MouseCameraLook
  (params (ActionValue :type Vector%202D%20Structure) (ElapsedSeconds :type Float%20%28double-precision%29) (TriggeredSeconds :type Float%20%28double-precision%29) (InputAction :type Input%20Action%20Object%20Reference :default "/Game/LAPLANQUE_ND/Inputs/Actions/IA_MouseCameraLook.IA_MouseCameraLook"))
  (if (and (Variables|Default|GetbCameraMovementActive) (Variables|/Game/LAPLANQUE_ND/UI/WBP_MainUI.WBP_MainUI_C|GetbIsMouseOverMainView (Variables|Default|GetMainUI)))
    (Pawn|Input|AddControllerYawInput (.x ActionValue))
    (Pawn|Input|AddControllerPitchInput (.y ActionValue))))

(event Input|EnhancedActionEvents|EnhancedInputActionIA_MouseCameraActivate
  (params (ActionValue :type Boolean) (ElapsedSeconds :type Float%20%28double-precision%29) (TriggeredSeconds :type Float%20%28double-precision%29) (InputAction :type Input%20Action%20Object%20Reference :default "/Game/LAPLANQUE_ND/Inputs/Actions/IA_MouseCameraActivate.IA_MouseCameraActivate"))
  (:Started
    (Variables|Default|SetbCameraMovementActive true))
  (:Completed
    (Variables|Default|SetbCameraMovementActive false)))

(event Input|EnhancedActionEvents|EnhancedInputActionIA_CharacterZMovement
  (params (ActionValue :type Float%20%28double-precision%29) (ElapsedSeconds :type Float%20%28double-precision%29) (TriggeredSeconds :type Float%20%28double-precision%29) (InputAction :type Input%20Action%20Object%20Reference :default "/Game/LAPLANQUE_ND/Inputs/Actions/IA_CharacterZMovement.IA_CharacterZMovement"))
  (if (Variables|/Game/LAPLANQUE_ND/UI/WBP_MainUI.WBP_MainUI_C|GetbIsMouseOverMainView (Variables|Default|GetMainUI))
    (Pawn|Input|AddMovementInput (Math|Vector|GetUpVector (Math|Rotator|MakeRotator (.roll (Pawn|GetControlRotation :!class /Script/Engine.Pawn)) 0.0 0.0)) ActionValue false)))

(event Input|EnhancedActionEvents|EnhancedInputActionIA_CharacterXYMovement
  (params (ActionValue :type Vector%202D%20Structure) (ElapsedSeconds :type Float%20%28double-precision%29) (TriggeredSeconds :type Float%20%28double-precision%29) (InputAction :type Input%20Action%20Object%20Reference :default "/Game/LAPLANQUE_ND/Inputs/Actions/IA_CharacterXYMovement.IA_CharacterXYMovement"))
  (bind _returnvalue (Pawn|GetControlRotation :!class /Script/Engine.Pawn))
  (if (Variables|/Game/LAPLANQUE_ND/UI/WBP_MainUI.WBP_MainUI_C|GetbIsMouseOverMainView (Variables|Default|GetMainUI))
    (Pawn|Input|AddMovementInput (Math|Vector|GetRightVector (Math|Rotator|MakeRotator (.roll _returnvalue) 0.0 (.yaw _returnvalue))) (.x ActionValue) false)
    (Pawn|Input|AddMovementInput (Math|Vector|GetForwardVector (Math|Rotator|MakeRotator 0.0 0.0 (.yaw _returnvalue))) (.y ActionValue) false)))

(event Input|EnhancedActionEvents|EnhancedInputActionIA_MouseCameraZoom
  (params (ActionValue :type Float%20%28double-precision%29) (ElapsedSeconds :type Float%20%28double-precision%29) (TriggeredSeconds :type Float%20%28double-precision%29) (InputAction :type Input%20Action%20Object%20Reference :default "/Game/LAPLANQUE_ND/Inputs/Actions/IA_MouseCameraZoom.IA_MouseCameraZoom"))
  (if (Variables|/Game/LAPLANQUE_ND/UI/WBP_MainUI.WBP_MainUI_C|GetbIsMouseOverMainView (Variables|Default|GetMainUI))
    (Variables|Default|SetSpringArmTargetLength (Math|Float|Clamp(Float) (+ (* ActionValue (Variables|Default|GetCameraZoomSpeed)) (Variables|/Script/Engine.SpringArmComponent|GetTargetArmLength (Variables|Default|GetSpringArm))) 2e+01 2e+03))))

(event EventBeginPlay
  (bind _returnvalue (Game|GetPlayerController 0))
  (bind _asplayer_controller (Utilities|Casting|CastToPlayerController (Pawn|GetController)))
  (Utilities|IsValid (PlayerController|LocalPlayerSubsystems|GetEnhancedInputLocalPlayerSubsystem _asplayer_controller)
    (:Is%20Valid
      (Input|AddMappingContext (PlayerController|LocalPlayerSubsystems|GetEnhancedInputLocalPlayerSubsystem _asplayer_controller) "/Game/LAPLANQUE_ND/Inputs/IMC_Controls.IMC_Controls" 0 "(bIgnoreAllPressedKeysUntilRelease=True,bForceImmediately=False,bNotifyUserSettings=False)")
      (bind _returnvalue_2 (UserInterface|CreateWidget "/Game/LAPLANQUE_ND/UI/WBP_MainUI.WBP_MainUI_C" (Game|GetPlayerController 0)))
      (bind _output_get (Variables|Default|SetMainUI _returnvalue_2))
      (UserInterface|Viewport|AddtoViewport _output_get 0)
      (Input|SetInputModeGameandUI _returnvalue (Variables|Default|GetMainUI) "DoNotLock" false false)
      (Variables|/Script/Engine.PlayerController|SetbShowMouseCursor _returnvalue true)
      (Variables|Default|SetSpringArmTargetLength (Variables|/Script/Engine.SpringArmComponent|GetTargetArmLength (Variables|Default|GetSpringArm)))
      (bind _outactors (Actor|GetAllActorsOfClass "/Game/LAPLANQUE_ND/Blueprints/UI/BP_ImGUI.BP_ImGUI_C"))
      (Variables|Default|SetImGUI (Utilities|Array|Get(acopy) _outactors)))))

(event EventTick
  (params (DeltaSeconds :type Float%20%28single-precision%29))
  (Variables|/Script/Engine.SpringArmComponent|SetTargetArmLength (Variables|Default|GetSpringArm) (Math|Interpolation|FInterpTo (Variables|/Script/Engine.SpringArmComponent|GetTargetArmLength (Variables|Default|GetSpringArm)) (Variables|Default|GetSpringArmTargetLength) DeltaSeconds 4.0))
  (bind _imgui (Variables|Default|GetImGUI)
    (:then
      (Variables|/Script/aKMcontrol.ImGuiActor|SetMainViewLocalTopLeft _imgui (Variables|/Game/LAPLANQUE_ND/UI/WBP_MainUI.WBP_MainUI_C|GetMainViewLocalTopLeft (Variables|Default|GetMainUI)))
      (Variables|/Script/aKMcontrol.ImGuiActor|SetMainViewLocalSize _imgui (Variables|/Game/LAPLANQUE_ND/UI/WBP_MainUI.WBP_MainUI_C|GetMainViewLocalSize (Variables|Default|GetMainUI)))
      (Variables|/Script/aKMcontrol.ImGuiActor|SetMainViewAbsoluteSize _imgui (Variables|/Game/LAPLANQUE_ND/UI/WBP_MainUI.WBP_MainUI_C|GetMainViewAbsoluteSize (Variables|Default|GetMainUI)))
      (Class|ImGuiActor|SetImGuiInput (Variables|Default|GetImGUI) (not (Variables|/Game/LAPLANQUE_ND/UI/WBP_MainUI.WBP_MainUI_C|GetbIsMouseOverMainView (Variables|Default|GetMainUI)))))
    (:else)))

(fn ConstructionScript)